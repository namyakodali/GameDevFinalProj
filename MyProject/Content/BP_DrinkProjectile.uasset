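; BP_DrinkProjectile is a drink projectile that damages and knocks back any first-person character entering its Sphere.
; On overlap it adds one to the character's Damage, launches it, then calls CheckDeath on it.
; The launch combines a normalized horizontal direction, from the projectile's Cylinder to its own actor location, with a fixed upward component, scaled to constant strength.
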(event OnComponentBeginOverlap(Sphere)
  (params (OverlappedComponent :type Primitive%20Component%20Object%20Reference) (OtherActor :type Actor%20Object%20Reference) (OtherComp :type Primitive%20Component%20Object%20Reference) (OtherBodyIndex :type Integer) (bFromSweep :type Boolean) (SweepResult :type Hit%20Result%20Structure%20%28by%20ref%29))
  (bind _returnvalue (Transformation|GetActorLocation))
  (bind _cylinder (Variables|Default|GetCylinder))
  (bind _returnvalue_2 (Transformation|GetWorldLocation _cylinder))
  (bind _returnvalue_3 (Math|Vector|GetUnitDirection(Vector) _returnvalue_2 _returnvalue))
  (bind _returnvalue_4 (Math|Vector|Normalize (Math|Vector|MakeVector (.x _returnvalue_3) (.y _returnvalue_3) 0.0)))
  (bind _asbp_first_person_character (Utilities|Casting|CastToBP_FirstPersonCharacter OtherActor))
  (Variables|/Game/FirstPerson/Blueprints/BP_FirstPersonCharacter.BP_FirstPersonCharacter_C|SetDamage _asbp_first_person_character (+ (Variables|/Game/FirstPerson/Blueprints/BP_FirstPersonCharacter.BP_FirstPersonCharacter_C|GetDamage _asbp_first_person_character) 1))
  (Character|LaunchCharacter _asbp_first_person_character (* (Math|Vector|MakeVector (.x _returnvalue_4) (.y _returnvalue_4) 1.0) 7e+02) false false)
  (Default|CheckDeath _asbp_first_person_character))

(event EventBeginPlay)

(event Collision|EventActorBeginOverlap
  (params (OtherActor :type Actor%20Object%20Reference)))

(event EventTick
  (params (DeltaSeconds :type Float%20%28single-precision%29)))

(fn ConstructionScript)